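; BP_Tower is a tower defense tower that can be selected, upgraded and sold.
; Clicking it registers it as BP_Core's selected tower and shows its camera-aligned context menu and detection range indicator.
; UpgradeTower spends gold through BP_GameModeTD to swap level meshes, double the next cost, raise sell value and fire OnUpgraded.
; SellTower refunds gold and destroys the actor, while helper functions adjust damage, fire rate and range.
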(event `self.ReceiveBeginPlay`
  (bind _towerdata (`self.TowerData`))
  (bind (_returnvalue_roll _returnvalue_pitch) (`KismetMathLibrary.BreakRotator` (`SceneComponent.K2_GetComponentRotation` (`PlayerCameraManager.TransformComponent` (`GameplayStatics.GetPlayerCameraManager` 0)))))
  (bind (_returnvalue_x _returnvalue_y) (`KismetMathLibrary.BreakVector` (`SceneComponent.K2_GetComponentLocation` (`PlayerCameraManager.TransformComponent` (`GameplayStatics.GetPlayerCameraManager` 0)))))
  (bind _asbp_core (cast `/Game/Blueprints/Player/BP_Core` (`GameplayStatics.GetPlayerPawn` 0)))
  (set `self.As BP Core` _asbp_core)
  (bind _asbp_game_mode_td (cast `/Game/Blueprints/GameMode/BP_GameModeTD` (`GameplayStatics.GetGameMode`)))
  (set `self.As BP Game Mode TD` _asbp_game_mode_td)
  (`SceneComponent.K2_SetWorldRotation` (`self.ContextMenu`) (`KismetMathLibrary.MakeRotator` 0.0 (* _returnvalue_pitch -1.0) 90.0) false false)
  (`SceneComponent.K2_SetWorldLocation` (`self.ContextMenu`) (`KismetMathLibrary.MakeVector` 0.0 (- _returnvalue_y -100.0) 1200.0) false false)
  (`/Engine/EditorBlueprintResources/StandardMacros.IsValid` _towerdata
    (:`Is Valid`
      (set `self.UpgradeCost` (* (`/Game/Blueprints/DataAssets/TowerDataAssets/PDA_TowerData.Cost` _towerdata) 2)))))

(event `self.ReceiveActorOnClicked`
  (params (ButtonPressed :type "Key Structure"))
  (bind _contextmenu (`self.ContextMenu`))
  (bind _contextmenu_2 (`self.ContextMenu`))
  (bind _contextmenu_3 (`self.ContextMenu`))
  (bind _sphereradius (`SphereComponent.SphereRadius` (`self.EnemyDetectCollision`)))
  (`KismetSystemLibrary.Delay` 0.01)
  (if (not (`SceneComponent.IsVisible` (`self.ContextMenu`)))
    (`/Engine/EditorBlueprintResources/StandardMacros.IsValid` (`/Game/Blueprints/Player/BP_Core.CurrentTowerSelected` (`self.As BP Core`))
      (:`Is Valid`
        ;[1 1 1] Hide previous Context menu then show current one
        (`SceneComponent.SetVisibility` _contextmenu_2 false false)
        (`PrimitiveComponent.SetCollisionResponseToChannel` _contextmenu_2 "ECC_Visibility" "ECR_Ignore")
        (set `/Game/Blueprints/Player/BP_Core.CurrentTowerSelected` self (`self.As BP Core`))
        (`SceneComponent.SetVisibility` _contextmenu true false)
        (`PrimitiveComponent.SetCollisionResponseToChannel` _contextmenu "ECC_Visibility" "ECR_Block"))
      (:`Is Not Valid`
        ;[1 1 1] Show context menu if none was showing
        (`SceneComponent.SetVisibility` _contextmenu_3 true false)
        (`PrimitiveComponent.SetCollisionResponseToChannel` _contextmenu_3 "ECC_Visibility" "ECR_Block")
        (set `/Game/Blueprints/Player/BP_Core.CurrentTowerSelected` self (`self.As BP Core`))))
    (`SceneComponent.SetVisibility` (`self.TowerRange`) true false)
    (`SceneComponent.SetWorldScale3D` (`self.TowerRange`) (`KismetMathLibrary.MakeVector` 200.0 _sphereradius _sphereradius))))

(fn `IncreaseDamage`
  (params (DamageUpgradeMultiplier :type "Float (double-precision)"))
  (set `self.Damage` (* (`self.Damage`) DamageUpgradeMultiplier)))

(fn `IncreaseFireRate`
  (params (FireRateMultiplier :type "Float (double-precision)"))
  (bind _output_get (set `self.FireRate` (/ (`self.FireRate`) FireRateMultiplier)))
  (set `self.DefaultFireRate` _output_get))

(fn `IncreaseRange`
  (params (AddToRange :type "Float (double-precision)"))
  (bind _enemydetectcollision (`self.EnemyDetectCollision`))
  (`SphereComponent.SetSphereRadius` _enemydetectcollision (+ (`SphereComponent.SphereRadius` _enemydetectcollision) AddToRange) true))

(fn `SellTower`
  (`/Game/Blueprints/GameMode/BP_GameModeTD.AddGold` (`self.As BP Game Mode TD`) (`self.SellCost`))
  (set `/Game/Blueprints/Player/BP_Core.CurrentTowerSelected` null (`self.As BP Core`))
  (`self.K2_DestroyActor`))

(fn `SwitchStaticMesh`
  (params (NewMesh :type "StaticMesh Object Reference") (InputPin :type "StaticMesh Object Reference"))
  (`StaticMeshComponent.SetStaticMesh` (`self.TowerBottom`) NewMesh)
  (`/Engine/EditorBlueprintResources/StandardMacros.IsValid` (`StaticMeshComponent.StaticMesh` (`self.TowerTop`))
    (:`Is Valid`
      (`StaticMeshComponent.SetStaticMesh` (`self.TowerTop`) InputPin))))

(fn `UpgradeTower`
  (bind (_basemesh _topmesh) (break `/Game/Blueprints/Towers/Struct_TowerMeshes` (`|GetArrayItem` (`self.StaticMeshesLevel`) (`self.Level`))))
  (if (>= (`/Game/Blueprints/Player/BP_Core.Gold` (`self.As BP Core`)) (`self.UpgradeCost`))
    (set `self.SellCost` (+ (`self.SellCost`) (/ (`self.UpgradeCost`) 2)))
    (`/Game/Blueprints/GameMode/BP_GameModeTD.DeductGold` (`self.As BP Game Mode TD`) (`self.UpgradeCost`))
    (`self.SwitchStaticMesh` _basemesh _topmesh)
    (set `self.UpgradeCost` (* (`self.UpgradeCost`) 2))
    (set `self.Level` (+ (`self.Level`) 1))
    (`self.OnUpgraded`)
    (if (== (`self.Level`) (`self.MaxLevel`))
      (set `self.IsMaxedUpgrade` true))))

(fn `UserConstructionScript`)