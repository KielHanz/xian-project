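; Missile tower that fires homing missiles at ground enemies and excludes flying ones from its targets.
; It extends a parent tower by binding to its shoot and upgrade events, pointing each projectile at the first enemy in range.
; Flying enemies are pruned from the in-range list on detection overlap and again at fire time.
; Upgrades multiply damage, fire rate and area-of-effect range.
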(event `self.ReceiveBeginPlay`
  (`parent.ReceiveBeginPlay`)
  (add `self.OnShoot` (delegate `OnTowerShoot`))
  (add `self.OnUpgraded` (delegate `Upgrade`)))

(event `OnTowerShoot` :!signature `self.OnShoot`
  (params (Projectile :type "Projectile Object Reference"))
  (bind _enemyinrangelist (`self.EnemyInRangeList`))
  (bind _output (`|GetArrayItem` (`self.EnemyInRangeList`)))
  (bind _output_2 (`|GetArrayItem` _enemyinrangelist))
  ;[1 1 1] Set Missile to be homing missile
  (if (not (`Enemy.IsFlyType` _output_2))
    (bind _asbp_missile_projectile (cast `/Game/Blueprints/Projectiles/BP_MissileProjectile` Projectile))
    (`/Engine/EditorBlueprintResources/StandardMacros.IsValid` _output
      (:`Is Valid`
        (`/Game/Blueprints/Projectiles/BP_MissileProjectile.SetHomingMissile` _asbp_missile_projectile self _output)))
    (else
      (`KismetArrayLibrary.Array_RemoveItem` _enemyinrangelist _output_2))))

(event `Upgrade`
  (`self.IncreaseDamage` 1.5)
  (`self.IncreaseFireRate` 1.5)
  (set `self.AreaOfEffectRange` (* (`self.AreaOfEffectRange`) 1.5)))

(event `self.EnemyDetectCollision.OnComponentBeginOverlap`
  (params (OverlappedComponent :type "PrimitiveComponent Object Reference") (OtherActor :type "Actor Object Reference") (OtherComp :type "PrimitiveComponent Object Reference") (OtherBodyIndex :type Integer) (bFromSweep :type Boolean) (SweepResult :type "HitResult Structure (by ref)"))
  ;[1 1 1] Remove air type if in enemy list
  (for _array_element (`PrimitiveComponent.GetOverlappingActors` (`self.EnemyDetectCollision`) "/Script/TDFinals_TRNDD.Enemy")
    (bind _asbp_enemy (cast `/Game/Blueprints/Enemies/BP_Enemy` _array_element))
    (if (`Enemy.IsFlyType` _asbp_enemy)
      (`KismetArrayLibrary.Array_RemoveItem` (`self.EnemyInRangeList`) _asbp_enemy))))

(fn `UserConstructionScript`
  (`parent.UserConstructionScript`))