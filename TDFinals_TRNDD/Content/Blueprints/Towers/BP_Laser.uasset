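; BP_Laser is a tower Blueprint that fires laser projectiles carrying burn damage.
; On BeginPlay it binds handlers to the inherited shoot and upgrade events.
; Each spawned BP_LaserProjectile receives the tower's current BurnDamage.
; Each upgrade scales damage, fire rate and burn damage by the same multiplier.
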(event `self.ReceiveBeginPlay`
  (`parent.ReceiveBeginPlay`)
  (add `Tower.OnShoot` (delegate `OnSpawnProjectile`))
  (add `self.OnUpgraded` (delegate `OnUpgrade`)))

(event `OnSpawnProjectile`
  (params (Projectile :type "Projectile Object Reference"))
  ;[1 1 1] Set Burn damage of laser projectile
  (bind _asbp_laser_projectile (cast `/Game/Blueprints/Projectiles/BP_LaserProjectile` Projectile))
  (set `/Game/Blueprints/Projectiles/BP_LaserProjectile.BurnDamage` (`self.BurnDamage`) _asbp_laser_projectile))

(event `OnUpgrade`
  (`self.IncreaseDamage` 1.5)
  (`self.IncreaseFireRate` 1.5)
  (set `self.BurnDamage` (* (`self.BurnDamage`) 1.5)))

(fn `UserConstructionScript`
  (`parent.UserConstructionScript`))