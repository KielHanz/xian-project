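; Homing missile projectile that deals area damage to non-flying enemies.
; SetHomingMissile copies damage and sphere radius from its owner and, given a valid enemy, homes the projectile movement on that enemy's mesh.
; When the missile mesh begins an overlap, it damages each overlapping ground BP_Enemy and spawns an explosion at its own location per hit.
; The graph never destroys the missile.
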(event `SetHomingMissile`
  (params (Owner :type "/Game/Blueprints/Towers/BP_Missile Object Reference") (Enemy :type "Enemy Object Reference"))
  (bind _projectilemovementcomponent (`self.ProjectileMovementComponent`))
  ;[1 1 1] Initialize Homing missile
  (set `self.BaseDamage` (`Tower.Damage` Owner))
  (`SphereComponent.SetSphereRadius` (`self.AreaOfEffect`) (`/Game/Blueprints/Towers/BP_Missile.AreaOfEffectRange` Owner) true)
  (`/Engine/EditorBlueprintResources/StandardMacros.IsValid` Enemy
    (:`Is Valid`
      (set `ProjectileMovementComponent.bIsHomingProjectile` true _projectilemovementcomponent)
      (set `ProjectileMovementComponent.HomingAccelerationMagnitude` 10000.0 _projectilemovementcomponent)
      (set `ProjectileMovementComponent.HomingTargetComponent` (`Enemy.StaticMesh` Enemy) _projectilemovementcomponent))))

(event `self.ProjectileMesh.OnComponentBeginOverlap`
  (params (OverlappedComponent :type "PrimitiveComponent Object Reference") (OtherActor :type "Actor Object Reference") (OtherComp :type "PrimitiveComponent Object Reference") (OtherBodyIndex :type Integer) (bFromSweep :type Boolean) (SweepResult :type "HitResult Structure (by ref)"))
  ;[1 1 1] AOE Damage but not on air types
  (for _array_element (`self.GetOverlappingActors` "/Game/Blueprints/Enemies/BP_Enemy.BP_Enemy_C")
    (bind _asbp_enemy (cast `/Game/Blueprints/Enemies/BP_Enemy` _array_element))
    (if (not (`Enemy.IsFlyType` _asbp_enemy))
      (`GameplayStatics.ApplyDamage` _asbp_enemy (`self.BaseDamage`))
      (`GameplayStatics.SpawnEmitterAtLocation` "/Game/StarterContent/Particles/P_Explosion.P_Explosion" (`self.K2_GetActorLocation`)))))

(fn `UserConstructionScript`)