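; Laser projectile that applies a burn debuff to any BP_Enemy its mesh begins overlapping.
; The burn is a BP_BurnEntity actor that receives the projectile's BurnDamage, attaches to the enemy and has its class registered in the enemy's DebuffList.
; On an already burning enemy, an attached burn of equal or lower damage is destroyed and respawned to reset it, while stronger burns remain.
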(event `self.ProjectileMesh.OnComponentBeginOverlap`
  (params (OverlappedComponent :type "PrimitiveComponent Object Reference") (OtherActor :type "Actor Object Reference") (OtherComp :type "PrimitiveComponent Object Reference") (OtherBodyIndex :type Integer) (bFromSweep :type Boolean) (SweepResult :type "HitResult Structure (by ref)"))
  ;[1 1 1] Adds the burning effect to enemies (resets every hit)
  (bind _asbp_enemy (cast `/Game/Blueprints/Enemies/BP_Enemy` OtherActor))
  (if (`KismetArrayLibrary.Array_Contains` (`/Game/Blueprints/Enemies/BP_Enemy.DebuffList` _asbp_enemy) "/Game/Blueprints/DebuffActors/BP_BurnEntity.BP_BurnEntity_C")
    (for _array_element (`self.GetAttachedActors` _asbp_enemy true false)
      (bind _asbp_burn_entity (cast `/Game/Blueprints/DebuffActors/BP_BurnEntity` _array_element))
      (if (<= (`/Game/Blueprints/DebuffActors/BP_BurnEntity.BurnDamage` _asbp_burn_entity) (`self.BurnDamage`))
        (if (== (`GameplayStatics.GetObjectClass` _array_element) "/Game/Blueprints/DebuffActors/BP_BurnEntity.BP_BurnEntity_C")
          (`self.K2_DestroyActor` _array_element)
          (bind _returnvalue (`|SpawnActorFromClass` "/Game/Blueprints/DebuffActors/BP_BurnEntity.BP_BurnEntity_C" (`KismetMathLibrary.MakeTransform` (0.0 0.0 0.0)) "Undefined" "MultiplyWithRoot" null null :!label _label))
          (set `/Game/Blueprints/DebuffActors/BP_BurnEntity.BurnDamage` (`self.BurnDamage`) _returnvalue)
          (`self.K2_AttachToActor` _returnvalue _asbp_enemy "None" "KeepRelative" "KeepRelative" "KeepRelative" true)
          (bind _debufflist (`/Game/Blueprints/Enemies/BP_Enemy.DebuffList` _asbp_enemy))
          (bind _returnvalue_2 (`GameplayStatics.GetObjectClass` _returnvalue))
          (if (not (`KismetArrayLibrary.Array_Contains` _debufflist _returnvalue_2))
            (`KismetArrayLibrary.Array_AddUnique` _debufflist _returnvalue_2)))))
    (else
      (goto _label))))

(fn `UserConstructionScript`)