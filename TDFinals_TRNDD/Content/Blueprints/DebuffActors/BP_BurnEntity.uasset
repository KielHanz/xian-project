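; A burn debuff actor that attaches to an enemy and deals periodic damage to it.
; BeginPlay starts a five-second lifetime timer and a self-recalling delay loop that damages the parent actor every half second.
; After a brief delay it binds to the parent BP_Enemy's destruction to destroy itself.
; On timeout it removes its class from the enemy's DebuffList and destroys itself.
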(event `self.ReceiveBeginPlay`
  (`KismetSystemLibrary.K2_SetTimerDelegate` (delegate `DestroyAfterTime`) 5.0)
  (`self.BurnLoop`)
  (`KismetSystemLibrary.Delay` 0.001)
  (bind _asbp_enemy (cast `/Game/Blueprints/Enemies/BP_Enemy` (`self.GetAttachParentActor`)))
  (add `self.OnDestroyed` _asbp_enemy (delegate `Destroy`)))

(event `Destroy` :!signature `self.OnDestroyed`
  (params (DestroyedActor :type "Actor Object Reference"))
  (`self.K2_DestroyActor`))

(event `DestroyAfterTime`
  (bind _asbp_enemy (cast `/Game/Blueprints/Enemies/BP_Enemy` (`self.GetAttachParentActor`))
    (:`then`
      (`KismetArrayLibrary.Array_RemoveItem` (`/Game/Blueprints/Enemies/BP_Enemy.DebuffList` _asbp_enemy) (`GameplayStatics.GetObjectClass` self)))
    (:`CastFailed`
      _))
  (`self.K2_DestroyActor`))

(event `BurnLoop`
  (`KismetSystemLibrary.Delay` 0.5)
  (`GameplayStatics.ApplyDamage` (`self.GetAttachParentActor`) (`self.BurnDamage`))
  (`self.BurnLoop`))

(fn `UserConstructionScript`)