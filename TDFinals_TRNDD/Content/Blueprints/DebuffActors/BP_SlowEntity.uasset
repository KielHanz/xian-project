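; BP_SlowEntity is a debuff actor that slows the BP_Enemy it is attached to.
; Shortly after BeginPlay it casts its attach parent to BP_Enemy and sets MaxWalkSpeed to the enemy's MoveSpeed divided by ReduceSpeedMultiplier.
; A handler bound to OnDestroyed restores the base speed and removes this actor's class from the enemy's DebuffList.
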(event `self.ReceiveBeginPlay`
  (`self.SlowEnemy`))

(event `SlowEnemy`
  (`KismetSystemLibrary.Delay` 0.01)
  (bind _asbp_enemy (cast `/Game/Blueprints/Enemies/BP_Enemy` (`self.GetAttachParentActor`)))
  (set `CharacterMovementComponent.MaxWalkSpeed` (/ (`Enemy.MoveSpeed` _asbp_enemy) (`self.ReduceSpeedMultiplier`)) (`Character.CharacterMovement` _asbp_enemy))
  (add `self.OnDestroyed` (delegate `OnRemoved`)))

(event `OnRemoved` :!signature `self.OnDestroyed`
  (params (DestroyedActor :type "Actor Object Reference"))
  (bind _asbp_enemy (cast `/Game/Blueprints/Enemies/BP_Enemy` (`self.GetAttachParentActor`)))
  (set `CharacterMovementComponent.MaxWalkSpeed` (`Enemy.MoveSpeed` _asbp_enemy) (`Character.CharacterMovement` _asbp_enemy))
  (`KismetArrayLibrary.Array_RemoveItem` (`/Game/Blueprints/Enemies/BP_Enemy.DebuffList` _asbp_enemy) (`GameplayStatics.GetObjectClass` self)))

(fn `UserConstructionScript`)