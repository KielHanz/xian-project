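; BP_Enemy is an enemy Blueprint that displays its health on a world-placed health bar widget.
; It refreshes the WB_EnemyHealth progress bar on BeginPlay and whenever the Health component reports damage, using current over maximum health.
; Each Tick, the bar pitches toward the player camera with roll and yaw held fixed, so it only partially billboards.
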(event `self.ReceiveBeginPlay`
  (`parent.ReceiveBeginPlay`)
  (add `HealthComponent.OnDamage` (`self.Health`) (delegate `UpdateHealthBar`))
  (`self.UpdateHealthBar`))

(event `UpdateHealthBar`
  (bind _health (`self.Health`))
  (bind _aswb_enemy_health (cast `/Game/Blueprints/Widgets/WB_EnemyHealth` (`WidgetComponent.GetWidget` (`self.HealthBar`))))
  (`ProgressBar.SetPercent` (`/Game/Blueprints/Widgets/WB_EnemyHealth.ProgressBar_0` _aswb_enemy_health) (/ (`KismetMathLibrary.Conv_IntToDouble` (`HealthComponent.CurrentHealth` _health)) (`KismetMathLibrary.Conv_IntToDouble` (`HealthComponent.MaxHealth` _health)))))

(event `self.ReceiveTick`
  (params (DeltaSeconds :type "Float (single-precision)"))
  (bind _healthbar (`self.HealthBar`))
  (bind (_returnvalue_roll _returnvalue_pitch) (`KismetMathLibrary.BreakRotator` (`KismetMathLibrary.FindLookAtRotation` (`SceneComponent.K2_GetComponentLocation` _healthbar) (`SceneComponent.K2_GetComponentLocation` (`PlayerCameraManager.TransformComponent` (`GameplayStatics.GetPlayerCameraManager` 0))))))
  (`parent.ReceiveTick` DeltaSeconds)
  (`SceneComponent.K2_SetWorldRotation` _healthbar (`KismetMathLibrary.MakeRotator` 0.0 _returnvalue_pitch 90.0) false false))

(fn `UserConstructionScript`)