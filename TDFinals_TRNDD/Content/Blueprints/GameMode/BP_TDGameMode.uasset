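; Tower defense game mode that runs enemy waves and creates the player HUD and game-over screen.
; WaveData defines each wave's enemy types, health and counts, which a self-retriggering one-second delay event spawns through BP_Spawner actors.
; Enemy death bindings count kills and start the next wave once the wave's total is reached.
; The BP_Core pawn's death shows the game-over widget; GiveGold is an empty stub.
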(event `self.ReceiveBeginPlay`
  (bind _asbp_core (cast `/Game/Blueprints/Player/BP_Core` (`GameplayStatics.GetPlayerPawn` 0)))
  (set `self.As BP Core` _asbp_core)
  (bind _returnvalue (`|GenericCreateObject` "/Game/Blueprints/Widgets/WB_PlayerUI.WB_PlayerUI_C"))
  (bind _output_get (set `self.PlayerUI Widget` _returnvalue))
  (`UserWidget.AddToViewport` _output_get 0)
  (`/Game/Blueprints/Widgets/WB_PlayerUI.UpdateHealthBar` _output_get)
  (`self.StartWave`)
  (add `HealthComponent.OnDeath` (`/Game/Blueprints/Player/BP_Core.Health` (`self.As BP Core`)) (delegate `OnPlayerDeath`)))

(event `OnPlayerDeath`
  (remove `HealthComponent.OnDeath` (`/Game/Blueprints/Player/BP_Core.Health` (`self.As BP Core`)) (delegate `OnPlayerDeath`))
  (bind _returnvalue (`|GenericCreateObject` "/Game/Blueprints/Widgets/WB_GameOver.WB_GameOver_C"))
  (`UserWidget.AddToViewport` _returnvalue 0))

(event `StartWave`
  ;[1 1 1] Starts the wave
  (if (< (`self.Waves`) (`KismetArrayLibrary.Array_Length` (`self.WaveData`)))
    (set `self.EnemyDataIdx` 0)
    (`self.SpawnEnemyDelay`)
    (set `self.EnemyDiedCount` 0)
    (`/Game/Blueprints/Widgets/WB_PlayerUI.UpdateWaveCount` (`self.PlayerUI Widget`))))

(event `SpawnEnemyDelay`
  (bind _enemydata (`WaveData.EnemyData` (`|GetArrayItem` (`self.WaveData`) (`self.Waves`))))
  (bind (_enemytype _hp _amountofenemies) (break `EnemyData` (`|GetArrayItem` _enemydata (`self.EnemyDataIdx`))))
  ;[1 1 1] Spawns specific enemy classes with delay
  (if (<= (`self.EnemyDataIdx`) (`KismetArrayLibrary.Array_Length` _enemydata))
    (`KismetSystemLibrary.Delay` 1.0)
    (bind _outactors (`GameplayStatics.GetAllActorsOfClass` "/Game/Blueprints/Spawner/BP_Spawner.BP_Spawner_C"))
    (for _array_element _outactors
      (bind _returnvalue (`Spawner.InitializeEnemySpawn` _array_element _enemytype (`KismetMathLibrary.FTrunc` _hp)))
      (`/Engine/EditorBlueprintResources/StandardMacros.IsValid` _returnvalue
        (:`Is Valid`
          (add `HealthComponent.OnDeath` (`Enemy.Health` _returnvalue) (delegate `OnEnemyDeath`)))
        (:`Is Not Valid`
          _))
      (set `self.EnemySpawnCount` (+ (`self.EnemySpawnCount`) 1))
      (`self.SpawnEnemyDelay`)
      (if (>= (`self.EnemySpawnCount`) _amountofenemies)
        (set `self.EnemySpawnCount` 0)
        (set `self.EnemyDataIdx` (+ (`self.EnemyDataIdx`) 1))))))

(event `CheckEnemies`
  ;[1 1 1] Checks enemies left and starts next wave if there is none left
  (set `self.EnemyWaveSpawnTotal` 0)
  (for _array_element (`WaveData.EnemyData` (`|GetArrayItem` (`self.WaveData`) (`self.Waves`)))
    (set `self.EnemyWaveSpawnTotal` (+ (`.AmountOfEnemies` (break `EnemyData` _array_element)) (`self.EnemyWaveSpawnTotal`))))
  (if (>= (`self.EnemyDiedCount`) (`self.EnemyWaveSpawnTotal`))
    (set `self.Waves` (+ (`self.Waves`) 1))
    (`self.StartWave`)))

(event `OnEnemyDeath`
  ;[1 1 1] Binded on every death of enemy (unbinds in c++ script of enemy)
  (`KismetSystemLibrary.PrintString` "Dead")
  (set `self.EnemyDiedCount` (+ (`self.EnemyDiedCount`) 1))
  (`self.CheckEnemies`))

(fn `GiveGold`)

(fn `UserConstructionScript`)