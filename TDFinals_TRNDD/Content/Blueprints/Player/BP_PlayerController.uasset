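; Player controller for a tower game that enables mouse cursor and click events and manages the selected tower's context menu.
; BeginPlay caches the player pawn as BP_Core, which holds the current tower selection.
; CheckOnClickContextMenu shows a hidden menu and makes it block Visibility traces.
; If the menu is already visible, a cursor trace missing it hides menu and range, ignores that channel, and deselects the tower.
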(event `self.ReceiveBeginPlay`
  (set `self.bShowMouseCursor` true)
  (set `self.bEnableClickEvents` true)
  (bind _asbp_core (cast `/Game/Blueprints/Player/BP_Core` (`GameplayStatics.GetPlayerPawn` 0)))
  (set `self.As BP Core` _asbp_core))

(event `CheckOnClickContextMenu`
  (bind _as_bp_core (`self.As BP Core`))
  (bind _currenttowerselected (`/Game/Blueprints/Player/BP_Core.CurrentTowerSelected` _as_bp_core))
  (bind _currenttowerselected_2 (`/Game/Blueprints/Player/BP_Core.CurrentTowerSelected` (`self.As BP Core`)))
  (bind _contextmenu (`/Game/Blueprints/Towers/BP_Tower.ContextMenu` _currenttowerselected))
  (bind _contextmenu_2 (`/Game/Blueprints/Towers/BP_Tower.ContextMenu` _currenttowerselected_2))
  (bind _contextmenu_3 (`/Game/Blueprints/Towers/BP_Tower.ContextMenu` (`/Game/Blueprints/Player/BP_Core.CurrentTowerSelected` (`self.As BP Core`))))
  (`/Engine/EditorBlueprintResources/StandardMacros.IsValid` _currenttowerselected_2
    (:`Is Valid`
      (if (not (`SceneComponent.IsVisible` _contextmenu_2))
        (`SceneComponent.SetVisibility` _contextmenu_3 true false)
        (`PrimitiveComponent.SetCollisionResponseToChannel` _contextmenu_3 "ECC_Visibility" "ECR_Block")
        (elif (not (== _contextmenu_2 (`.HitComponent` (`GameplayStatics.BreakHitResult` (`self.GetHitResultUnderCursorByChannel` "TraceTypeQuery1")))))
          (`SceneComponent.SetVisibility` _contextmenu false false)
          (`PrimitiveComponent.SetCollisionResponseToChannel` _contextmenu "ECC_Visibility" "ECR_Ignore")
          (`SceneComponent.SetVisibility` (`/Game/Blueprints/Towers/BP_Tower.TowerRange` _currenttowerselected) false false)
          (set `/Game/Blueprints/Player/BP_Core.CurrentTowerSelected` null _as_bp_core))))))

(fn `UserConstructionScript`)