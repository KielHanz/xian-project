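; BP_SubCores is a sub-core in the tower defense game that turns enemy contact into damage on the player's BP_Core pawn.
; When an enemy overlaps its static mesh, it deals that enemy damage equal to its max health.
; A boss costs the core its full max health, while other enemies deal a small fixed amount.
; The game mode's player UI health bar refresh is called before either damage is applied.
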(event `self.StaticMesh.OnComponentBeginOverlap`
  (params (OverlappedComponent :type "PrimitiveComponent Object Reference") (OtherActor :type "Actor Object Reference") (OtherComp :type "PrimitiveComponent Object Reference") (OtherBodyIndex :type Integer) (bFromSweep :type Boolean) (SweepResult :type "HitResult Structure (by ref)"))
  (bind _asenemy (cast `Enemy` OtherActor))
  (bind _asbp_game_mode_td (cast `/Game/Blueprints/GameMode/BP_GameModeTD` (`GameplayStatics.GetGameMode`)))
  (`/Game/Blueprints/Widgets/WB_PlayerUI.UpdateHealthBar` (`/Game/Blueprints/GameMode/BP_GameModeTD.PlayerUI Widget` _asbp_game_mode_td))
  (`GameplayStatics.ApplyDamage` _asenemy (`KismetMathLibrary.Conv_IntToDouble` (`HealthComponent.MaxHealth` (`Enemy.Health` _asenemy))))
  (cast `/Game/Blueprints/Enemies/BP_Enemy_Boss` _asenemy
    (:`then`
      (bind _asbp_core (cast `/Game/Blueprints/Player/BP_Core` (`GameplayStatics.GetPlayerPawn` 0)))
      (`GameplayStatics.ApplyDamage` _asbp_core (`KismetMathLibrary.Conv_IntToDouble` (`HealthComponent.MaxHealth` (`/Game/Blueprints/Player/BP_Core.Health` _asbp_core)))))
    (:`CastFailed`
      (bind _asbp_core_2 (cast `/Game/Blueprints/Player/BP_Core` (`GameplayStatics.GetPlayerPawn` 0)))
      (`GameplayStatics.ApplyDamage` _asbp_core_2 5.0))))

(fn `UserConstructionScript`)