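; BP_SalvageEntity is a debuff actor attached to an enemy that awards gold to the player when that enemy dies.
; Shortly after BeginPlay, it binds to the parent enemy's Health death event, which adds GoldGiven through BP_GameModeTD.
; It destroys itself when the enemy is destroyed, and on its own destruction unbinds the death event and removes its class from the enemy's DebuffList.
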(event `self.ReceiveBeginPlay`
  (`KismetSystemLibrary.Delay` 0.01)
  (bind _asbp_enemy (cast `/Game/Blueprints/Enemies/BP_Enemy` (`self.GetAttachParentActor`)))
  (add `HealthComponent.OnDeath` (`Enemy.Health` _asbp_enemy) (delegate `SalvageEnemy`))
  (add `self.OnDestroyed` (delegate `OnRemove`))
  (`KismetSystemLibrary.Delay` 0.001)
  (bind _asenemy (cast `Enemy` (`self.GetAttachParentActor`)))
  (add `self.OnDestroyed` _asenemy (delegate `Destroy`)))

(event `Destroy` :!signature `self.OnDestroyed`
  (params (DestroyedActor :type "Actor Object Reference"))
  (`self.K2_DestroyActor`))

(event `OnRemove` :!signature `self.OnDestroyed`
  (params (DestroyedActor :type "Actor Object Reference"))
  (bind _asbp_enemy (cast `/Game/Blueprints/Enemies/BP_Enemy` (`self.GetAttachParentActor`)))
  (remove `HealthComponent.OnDeath` (`Enemy.Health` _asbp_enemy) (delegate `SalvageEnemy`))
  (`KismetArrayLibrary.Array_RemoveItem` (`/Game/Blueprints/Enemies/BP_Enemy.DebuffList` _asbp_enemy) (`GameplayStatics.GetObjectClass` self)))

(event `SalvageEnemy`
  (bind _asbp_game_mode_td (cast `/Game/Blueprints/GameMode/BP_GameModeTD` (`GameplayStatics.GetGameMode`)))
  (`/Game/Blueprints/GameMode/BP_GameModeTD.AddGold` _asbp_game_mode_td (`self.GoldGiven`)))

(fn `UserConstructionScript`)