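; Overload buff actor that changes the fire rate of the BP_Tower it is attached to.
; After a brief delay on BeginPlay it sets the tower's FireRate to DefaultFireRate divided by AttackSpeedBonus.
; It destroys itself when the tower is destroyed.
; On its own destruction it restores the default rate and removes its class from the tower's BuffList.
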(event `self.ReceiveBeginPlay`
  (add `self.OnDestroyed` (delegate `OnRemoved`))
  (`self.SetFireRate`)
  (`KismetSystemLibrary.Delay` 0.001)
  (bind _asbp_tower (cast `/Game/Blueprints/Towers/BP_Tower` (`self.GetAttachParentActor`)))
  (add `self.OnDestroyed` _asbp_tower (delegate `OnTowerSold`)))

(event `OnTowerSold` :!signature `self.OnDestroyed`
  (params (DestroyedActor :type "Actor Object Reference"))
  (`self.K2_DestroyActor`))

(event `OnRemoved` :!signature `self.OnDestroyed`
  (params (DestroyedActor :type "Actor Object Reference"))
  (bind _asbp_tower (cast `/Game/Blueprints/Towers/BP_Tower` (`self.GetAttachParentActor`)))
  (set `Tower.FireRate` (`Tower.DefaultFireRate` _asbp_tower) _asbp_tower)
  (`KismetArrayLibrary.Array_RemoveItem` (`/Game/Blueprints/Towers/BP_Tower.BuffList` _asbp_tower) (`GameplayStatics.GetObjectClass` self)))

(event `SetFireRate`
  (`KismetSystemLibrary.Delay` 0.01)
  (bind _asbp_tower (cast `/Game/Blueprints/Towers/BP_Tower` (`self.GetAttachParentActor`)))
  (set `Tower.FireRate` (/ (`Tower.DefaultFireRate` _asbp_tower) (`self.AttackSpeedBonus`)) _asbp_tower))

(fn `UserConstructionScript`)